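; Collectable pickup actor that adds one of its item to a player's inventory on touch.
; When a BP_PlayerBase overlaps its collision, it wraps its item structure in a slot and passes it to that player's InventoryComponent.
; If the add succeeds, it destroys itself, then notifies every quest in player character 0's QuestLog of the collected item, passing itself along.
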(event `self.Collision.OnComponentBeginOverlap`
  (params (OverlappedComponent :type "PrimitiveComponent Object Reference") (OtherActor :type "Actor Object Reference") (OtherComp :type "PrimitiveComponent Object Reference") (OtherBodyIndex :type Integer) (bFromSweep :type Boolean) (SweepResult :type "HitResult Structure (by ref)"))
  (bind _asbp_player_base (cast `/Game/Blueprints/BP_PlayerBase` OtherActor))
  (bind _success (`/Game/InventorySystem/InventoryComponent.AddToInventory` (`/Game/Blueprints/BP_PlayerBase.InventoryComponent` _asbp_player_base) (make `/Game/InventorySystem/SlotStructure` (`self.ItemStructure`) 1)))
  (if _success
    (`self.K2_DestroyActor` self)
    (bind _asbp_player_base_2 (cast `/Game/Blueprints/BP_PlayerBase` (`GameplayStatics.GetPlayerCharacter` 0)))
    (for _array_element (`/Game/QuestSystem/QuestLog.Quests` (`/Game/Blueprints/BP_PlayerBase.QuestLog` _asbp_player_base_2))
      (`/Game/QuestSystem/Quests/Quest.CollectedItem` _array_element self))))

(fn `UserConstructionScript`)