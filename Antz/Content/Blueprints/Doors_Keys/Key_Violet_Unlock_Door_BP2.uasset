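; Violet key pickup that records itself as collected in the KeyTracker game instance.
; Overlapping its box as BP_PlayerBase shows an InteractUI prompt, enables input and opens a gate; leaving reverses this.
; Pressing Interact through the open gate sets the VioletKey flag, plays a pickup sound and destroys the actor.
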(event `InputAction|Interact`
  (params (Key :type "Key Structure"))
  (:`Pressed`
    (`/Engine/EditorBlueprintResources/StandardMacros.Gate` true :!label _label
      (:`Exit`
        (bind _askey_tracker (cast `/Game/Blueprints/KeyTracker` (`GameplayStatics.GetGameInstance`)))
        (set `/Game/Blueprints/KeyTracker.Violet Key` true _askey_tracker)
        (`GameplayStatics.PlaySoundAtLocation` "/Game/Audio/Interactables/Key_Pickup/Key_Pickup_Cue.Key_Pickup_Cue" (`self.K2_GetActorLocation`) (struct) 1.0 1.0 0.0 null null null)
        (`self.K2_DestroyActor`)))))

(event `self.Box.OnComponentBeginOverlap`
  (params (OverlappedComponent :type "PrimitiveComponent Object Reference") (OtherActor :type "Actor Object Reference") (OtherComp :type "PrimitiveComponent Object Reference") (OtherBodyIndex :type Integer) (bFromSweep :type Boolean) (SweepResult :type "HitResult Structure (by ref)"))
  (cast `/Game/Blueprints/BP_PlayerBase` OtherActor)
  (bind _returnvalue (`|CreateWidget` "/Game/QuestSystem/QuestUI/InteractUI.InteractUI_C"))
  (`UserWidget.AddToViewport` _returnvalue 0)
  (`self.EnableInput` (`GameplayStatics.GetPlayerController` 0))
  (goto _label :!via `Open`))

(event `self.Box.OnComponentEndOverlap`
  (params (OverlappedComponent :type "PrimitiveComponent Object Reference") (OtherActor :type "Actor Object Reference") (OtherComp :type "PrimitiveComponent Object Reference") (OtherBodyIndex :type Integer))
  (cast `/Game/Blueprints/BP_PlayerBase` OtherActor)
  (`self.DisableInput` (`GameplayStatics.GetPlayerController` 0))
  (`Widget.RemoveFromParent` (stale `self.Box.OnComponentBeginOverlap` _returnvalue))
  (goto _label :!via `Close`))

(fn `UserConstructionScript`)