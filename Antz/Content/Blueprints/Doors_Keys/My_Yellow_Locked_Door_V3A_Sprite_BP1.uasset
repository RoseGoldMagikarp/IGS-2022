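; A yellow locked sprite door that disappears when a player holding the yellow key interacts with it.
; Entering its box enables input and shows an interact prompt; interacting without the key shows a rejection widget.
; Leaving disables input and removes both widgets plus the player's quest log UI.
; The construction script writes sprite scale into a burn material parameter collection's Location and Scale, but the unlock burn call is never run.
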(event `self.Box.OnComponentBeginOverlap`
  (params (OverlappedComponent :type "PrimitiveComponent Object Reference") (OtherActor :type "Actor Object Reference") (OtherComp :type "PrimitiveComponent Object Reference") (OtherBodyIndex :type Integer) (bFromSweep :type Boolean) (SweepResult :type "HitResult Structure (by ref)"))
  (bind _asbp_player_base (cast `/Game/Blueprints/BP_PlayerBase` OtherActor))
  (`self.EnableInput` (`GameplayStatics.GetPlayerController` 0))
  (bind _returnvalue (`|CreateWidget` "/Game/QuestSystem/QuestUI/InteractUI.InteractUI_C"))
  (`UserWidget.AddToViewport` _returnvalue 0))

(event `InputAction|Interact`
  (params (Key :type "Key Structure"))
  (:`Pressed`
    (if (== (`/Game/Blueprints/BP_PlayerBase.Has Yellow Key?` (stale `self.Box.OnComponentBeginOverlap` _asbp_player_base)) true)
      (`self.K2_DestroyActor`)
      (else
        (bind _returnvalue (`|CreateWidget` "/Game/Blueprints/Doors_Keys/No_Key_Door_Rejection_Text_Widget.No_Key_Door_Rejection_Text_Widget_C"))
        (`UserWidget.AddToViewport` _returnvalue 0)))))

(event `self.Box.OnComponentEndOverlap`
  (params (OverlappedComponent :type "PrimitiveComponent Object Reference") (OtherActor :type "Actor Object Reference") (OtherComp :type "PrimitiveComponent Object Reference") (OtherBodyIndex :type Integer))
  (bind _asbp_player_base (cast `/Game/Blueprints/BP_PlayerBase` OtherActor))
  (`self.DisableInput` (`GameplayStatics.GetPlayerController` 0))
  (`WidgetBlueprintLibrary.GetAllWidgetsOfClass` "/Game/Blueprints/Doors_Keys/No_Key_Door_Rejection_Text_Widget.No_Key_Door_Rejection_Text_Widget_C")
  (`WidgetBlueprintLibrary.GetAllWidgetsOfClass` "/Game/QuestSystem/QuestUI/InteractUI.InteractUI_C")
  (`Widget.RemoveFromParent` (stale `InputAction|Interact` _returnvalue))
  (`Widget.RemoveFromParent` (`/Game/Blueprints/BP_PlayerBase.QuestLogUI` _asbp_player_base))
  (`Widget.RemoveFromParent` (stale `self.Box.OnComponentBeginOverlap` _returnvalue)))

(fn `Is Input Key Down?`
  (params (PlayerIndex :type Integer))
  (returns (ReturnValue :type Boolean))
  (return (`PlayerController.IsInputKeyDown` (`GameplayStatics.GetPlayerController` PlayerIndex) "X")))

(fn `UserConstructionScript`
  (bind _returnvalue (`SceneComponent.K2_GetComponentScale` (`self.PaperSprite`)))
  (`KismetMaterialLibrary.SetVectorParameterValue` "/Game/Blueprints/Doors_Keys/Burning_My_Locked_Door_V3A_Mat.Burning_My_Locked_Door_V3A_Mat" "Location" (`KismetMathLibrary.Conv_VectorToLinearColor` _returnvalue))
  (`KismetMaterialLibrary.SetVectorParameterValue` "/Game/Blueprints/Doors_Keys/Burning_My_Locked_Door_V3A_Mat.Burning_My_Locked_Door_V3A_Mat" "Scale" (`KismetMathLibrary.Conv_VectorToLinearColor` _returnvalue)))