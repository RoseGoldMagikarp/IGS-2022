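; Dialog component that runs a behavior-tree-driven conversation when a player interacts with it.
; On begin play it spawns a dedicated AI controller, using the behavior tree as a dialog flow engine.
; Interact shows a dialog widget with UI-only input, starts the dialog tree and passes the widget to it through the blackboard.
; The widget's exit event restores game input, stops the tree and removes the widget.
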(event `self.ReceiveBeginPlay`
  (bind _returnvalue (`|SpawnActorFromClass` "/Game/Blueprints/Dialog_System/Dialog_AI_Controler.Dialog_AI_Controler_C" (`KismetMathLibrary.MakeTransform` (0.0 0.0 0.0)) "Undefined" "OverrideRootScale" null null))
  (set `self.AI Controller` _returnvalue))

(event `/Game/Assets/Doors_and_Levers/Interact_Interface.Interact`
  (params (Player :type "Character Object Reference"))
  (bind _asplayer_controller (cast `PlayerController` (`Pawn.GetController` Player)))
  (bind _returnvalue (`|CreateWidget` "/Game/Blueprints/Dialog_System/Dialog_Widget.Dialog_Widget_C"))
  (bind _output_get (set `self.Dialog Widget` _returnvalue))
  (add `/Game/Blueprints/Dialog_System/Dialog_Widget.On Exit` _output_get (delegate `On Exit_Event_0`))
  (`UserWidget.AddToViewport` _output_get 0)
  (`WidgetBlueprintLibrary.SetInputMode_UIOnlyEx` _asplayer_controller _output_get)
  (set `PlayerController.bShowMouseCursor` true _asplayer_controller)
  (`AIController.RunBehaviorTree` (`self.AI Controller`) (`self.Dialog Tree`))
  (bind _blackboardcomponent (`AIController.UseBlackboard` (`self.AI Controller`) "/Game/Blueprints/Dialog_System/Dialog_BlackBoard.Dialog_BlackBoard"))
  (`BlackboardComponent.SetValueAsObject` _blackboardcomponent "Dialog Widget" (`self.Dialog Widget`)))

(event `On Exit_Event_0`
  (bind _returnvalue (`Widget.GetOwningPlayer` (`self.Dialog Widget`)))
  (`WidgetBlueprintLibrary.SetInputMode_GameOnly` _returnvalue)
  (set `PlayerController.bShowMouseCursor` false _returnvalue)
  (`BrainComponent.StopLogic` (`AIController.BrainComponent` (`self.AI Controller`)) "Dialog Exited")
  (`Widget.RemoveFromParent` (`self.Dialog Widget`)))