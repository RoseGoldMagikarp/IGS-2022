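; NPC dialog Blueprint that shows an interact prompt when the player is near, with placeholder dialog logic.
; A Box trigger shows its TextRender when a BP_PlayerBase overlaps and hides it on exit.
; A custom event, with no caller in this graph, prints a greeting, switches player 0 to UI-only input through PlayerAdjustments and hides the prompt.
; No dialog widget or input restore is present.
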(event `self.Box.OnComponentBeginOverlap`
  (params (OverlappedComponent :type "PrimitiveComponent Object Reference") (OtherActor :type "Actor Object Reference") (OtherComp :type "PrimitiveComponent Object Reference") (OtherBodyIndex :type Integer) (bFromSweep :type Boolean) (SweepResult :type "HitResult Structure (by ref)"))
  ;[1 1 1] Show Interact
  (cast `/Game/Blueprints/BP_PlayerBase` OtherActor)
  (`SceneComponent.SetHiddenInGame` (`self.TextRender`) false false))

(event `self.Box.OnComponentEndOverlap`
  (params (OverlappedComponent :type "PrimitiveComponent Object Reference") (OtherActor :type "Actor Object Reference") (OtherComp :type "PrimitiveComponent Object Reference") (OtherBodyIndex :type Integer))
  ;[1 1 1] Show Interact
  (cast `/Game/Blueprints/BP_PlayerBase` OtherActor)
  (`SceneComponent.SetHiddenInGame` (`self.TextRender`) true false))

(event `CustomEvent`
  (`KismetSystemLibrary.PrintString` "Hello")
  (`self.PlayerAdjustments`)
  (`SceneComponent.SetHiddenInGame` (`self.TextRender`) true false))

(event `PlayerAdjustments`
  (`WidgetBlueprintLibrary.SetInputMode_UIOnlyEx` (`GameplayStatics.GetPlayerController` 0) null))

(fn `UserConstructionScript`)